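; Player-controlled Apache helicopter that moves, yaws and fires paired rockets from left and right spawn points, with both explosion effects at the left one.
; Axis inputs feed a shared FInterpTo helper for smoothed local movement and key-driven yaw.
; Mouse yaw applies directly, and both turn inputs bank the spring arm with clamped roll.
; A timeline with no wired trigger holds the main and tail rotor spin.
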(fn ConstructionScript)

(fn 선형보간
  (params (AxisValue :type Float%20%28single-precision%29) (Current :type Float%20%28single-precision%29) (Speed :type Float%20%28single-precision%29))
  (bind _returnvalue (Utilities|Time|GetWorldDeltaSeconds))
  (return (Math|Interpolation|FInterpTo Current (* AxisValue Speed _returnvalue) _returnvalue 6.0)))

(event Input|AxisEvents|InputAxis앞뒤이동
  (params (AxisValue :type Float%20%28single-precision%29))
  (bind _returnvalue (CallFunction|선형보간 AxisValue (Variables|Default|GetCurrentX) (Variables|Default|GetSpeedMove)))
  (bind _output_get (Variables|Default|SetCurrentX _returnvalue))
  (Transformation|AddActorLocalOffset (Math|Vector|MakeVector _output_get 0.0 0.0) false false))

(event Input|AxisEvents|InputAxis좌우이동
  (params (AxisValue :type Float%20%28single-precision%29))
  (bind _returnvalue (CallFunction|선형보간 AxisValue (Variables|Default|GetCurrentY) (Variables|Default|GetSpeedMove)))
  (bind _output_get (Variables|Default|SetCurrentY _returnvalue))
  (Transformation|AddActorLocalOffset (Math|Vector|MakeVector 0.0 _output_get 0.0) false false))

(event Input|AxisEvents|InputAxis위아래이동
  (params (AxisValue :type Float%20%28single-precision%29))
  (bind _returnvalue (CallFunction|선형보간 AxisValue (Variables|Default|GetCurrentZ) (Variables|Default|GetSpeedMove)))
  (bind _output_get (Variables|Default|SetCurrentZ _returnvalue))
  (Transformation|AddActorLocalOffset (Math|Vector|MakeVector 0.0 0.0 _output_get) false false))

(event Input|AxisEvents|InputAxis마우스좌우회전
  (params (AxisValue :type Float%20%28single-precision%29))
  (Transformation|AddActorLocalRotation (Math|Rotator|MakeRotator 0.0 0.0 AxisValue) false false)
  (Variables|Default|SetArmRoll (Math|Float|Clamp(Float) (- (Variables|Default|GetArmRoll) AxisValue) -15.0 15.0))
  (Transformation|SetWorldRotation (Variables|Default|GetSpringArm) (Math|Rotator|MakeRotator (Math|Float|Clamp(Float) (- (Variables|Default|GetArmRoll) AxisValue) -15.0 15.0) (Variables|Default|GetArmPitch) (+ (.Yaw (Math|Rotator|BreakRotator (Transformation|GetActorRotation))) (Variables|Default|GetArmYaw))) false false))

(event Input|AxisEvents|InputAxis좌우회전
  (params (AxisValue :type Float%20%28single-precision%29))
  (bind _returnvalue (CallFunction|선형보간 AxisValue (Variables|Default|GetCurrentYaw) (Variables|Default|GetSpeedRot)))
  (bind _output_get (Variables|Default|SetCurrentYaw _returnvalue))
  (Transformation|AddActorLocalRotation (Math|Rotator|MakeRotator 0.0 0.0 _output_get) false false)
  (bind _returnvalue_2 (CallFunction|선형보간 AxisValue (Variables|Default|GetArmRoll) -1.5e+03))
  (Variables|Default|SetArmRoll (Math|Float|Clamp(Float) _returnvalue_2 -15.0 15.0))
  (Transformation|SetWorldRotation (Variables|Default|GetSpringArm) (Math|Rotator|MakeRotator (Variables|Default|GetArmRoll) (Variables|Default|GetArmPitch) (.Yaw (Math|Rotator|BreakRotator (Transformation|GetActorRotation)))) false false))

(event Input|ActionEvents|InputAction발사
  (params (Key :type Key%20Structure :default "None"))
  (bind _spawnright (Variables|Default|GetSpawnRight))
  (bind _spawnleft (Variables|Default|GetSpawnLeft))
  (bind _returnvalue (Transformation|GetWorldTransform _spawnleft))
  (bind _returnvalue_2 (Transformation|GetWorldTransform _spawnright))
  (:Pressed
    (Utilities|FlowControl|Sequence
      (:then_0
        (Game|SpawnActorfromClass "/Game/Apache/Blueprints/Rocket_BP.Rocket_BP_C" _returnvalue "Undefined" 0 0)
        (Effects|SpawnEmitteratLocation "/Game/Apache/Effects/P_Explosion_1.P_Explosion_1" (Math|Transform|TransformLocation _returnvalue "0, 0, 0")))
      (:then_1
        (Game|SpawnActorfromClass "/Game/Apache/Blueprints/Rocket_BP.Rocket_BP_C" _returnvalue_2 "Undefined" 0 0)
        (Effects|SpawnEmitteratLocation "/Game/Apache/Effects/P_Explosion_1.P_Explosion_1" (Math|Transform|TransformLocation _returnvalue_2 "0, 0, 0"))))))